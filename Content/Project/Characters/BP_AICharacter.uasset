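; AI character Blueprint that shows a cursor decal for hover and selection, styled by its attitude towards the player.
; Mesh cursor-over shows the decal with a hovered material, and the Selected event sets visibility and applies the selected material.
; Both materials are picked per Hostile, Neutral or UnderControl attitude.
; When the cursor leaves, the decal stays visible only if selected, without switching its material back.
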(fn ConstructionScript)

(fn SetDecalVisibility
  (params (Is%20Visible :type Boolean))
  (Rendering|SetVisibility (Variables|Default|GetDecal) Is%20Visible false))

(fn SetDecalHoweredMaterial
  (Rendering|Components|Decal|SetDecalMaterial (Variables|Default|GetDecal) (Utilities|Select :Index (Variables|Default|GetAttitudeTowardsPlayer) :Hostile "/Game/Project/Cursor/SelectionDecal/MI_CursorDecal_Hostile_Hovered.MI_CursorDecal_Hostile_Hovered" :Neutral "/Game/Project/Cursor/SelectionDecal/MI_CursorDecal_Neutral_Hovered.MI_CursorDecal_Neutral_Hovered" :Under_Control "/Game/Project/Cursor/SelectionDecal/MI_CursorDecal_UnderControl_Hovered.MI_CursorDecal_UnderControl_Hovered")))

(fn SetDecalSelectedMaterial
  (Rendering|Components|Decal|SetDecalMaterial (Variables|Default|GetDecal) (Utilities|Select :Index (Variables|Default|GetAttitudeTowardsPlayer) :Hostile "/Game/Project/Cursor/SelectionDecal/MI_CursorDecal_Hostile.MI_CursorDecal_Hostile" :Neutral "/Game/Project/Cursor/SelectionDecal/MI_CursorDecal_Neutral.MI_CursorDecal_Neutral" :Under_Control "/Game/Project/Cursor/SelectionDecal/MI_CursorDecal_UnderControl.MI_CursorDecal_UnderControl")))

(event OnBeginCursorOver(Mesh)
  (params (TouchedComponent :type Primitive%20Component%20Object%20Reference))
  ;[1 1 1] Mouse Cursor Over
  (Decal|SetDecalVisibility true)
  (Decal|SetDecalHoweredMaterial))

(event OnEndCursorOver(Mesh)
  (params (TouchedComponent :type Primitive%20Component%20Object%20Reference))
  ;[1 1 1] Mouse Cursor Over
  (Decal|SetDecalVisibility (stale EventSelected IsSelected)))

(event EventSelected
  (params (IsSelected :type Boolean))
  (Decal|SetDecalVisibility IsSelected)
  (Decal|SetDecalSelectedMaterial))