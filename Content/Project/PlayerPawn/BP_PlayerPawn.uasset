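; BP_PlayerPawn is the player pawn, which sets up the game HUD and exposes the party inventory toggle.
; On BeginPlay it creates WBP_HUD and adds it to the viewport.
; After a short delay it calls Interact on the first BP_Container_Base found in the level, without any player input.
; The ToggleInventory event forwards to PartyInventory.
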(event EventToggleInventory
  (Class|InventoryComponent|ToggleInventory (Variables|Default|GetParty%20Inventory) 0))

(fn ConstructionScript)

(fn InitializeGameHUD
  (bind _returnvalue (UserInterface|CreateWidget "/Game/Project/UI/HUD/WBP_HUD.WBP_HUD_C"))
  (UserInterface|Viewport|AddtoViewport _returnvalue 0))

(event EventBeginPlay
  (CallFunction|InitializeGameHUD)
  (Utilities|FlowControl|Delay 2.0)
  (bind _outactors (Actor|GetAllActorsOfClass "/Game/Project/Containers/BP_Container_Base.BP_Container_Base_C"))
  (Class|InteractableActor|Interact (Utilities|Array|Get(acopy) _outactors)))