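; BP_InventoryComponent is an inventory component that holds slot items with quantities and opens or closes the inventory panel.
; ToggleInventory removes the existing panel, or creates WBP_InventoryPanel with itself as PlayerInventory plus the given Container and adds it to the viewport.
; RefreshInventory rewrites each slot that has a valid item class from that class's defaults, keeping its quantity.
; Both events delegate to implementation functions.
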(event EventRefreshInventory
  (CallFunction|RefreshInventoryImplementation))

(event EventToggleInventory
  (params (Container :type Inventory%20Component%20Object%20Reference))
  (CallFunction|ToggleInventoryImplementation Container))

(fn RefreshInventoryImplementation
  (for (_array_element _array_index) (Variables|Default|GetInventory)
    (if (Utilities|IsValidClass (Utilities|Struct|BreakItem (.slotitem _array_element)))
      (Utilities|Array|SetArrayElem (Variables|Default|GetInventory) _array_index (Utilities|Struct|MakeSlot (Utilities|GetClassDefaults (Utilities|Struct|BreakItem (.slotitem _array_element))) (.slotquantity _array_element))))))

(fn ToggleInventoryImplementation
  (params (Container :type Inventory%20Component%20Object%20Reference))
  (bind _inventorywidget (Variables|Default|GetInventoryWidget)
    (:then
      (Widget|RemovefromParent _inventorywidget)
      (Variables|Default|SetInventoryWidget 0))
    (:else
      (bind _returnvalue (UserInterface|CreateWidget "/Game/Project/UI/Inventory/WBP_InventoryPanel.WBP_InventoryPanel_C" 0 self Container))
      (bind _output_get (Variables|Default|SetInventoryWidget _returnvalue))
      (UserInterface|Viewport|AddtoViewport _output_get 0))))